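; AugeBP is an eye actor that watches the player while its Trigger is triggered and the referenced Axt is alive (Lebendig).
; When following, Tick eases the Pivot toward the look-at yaw and maps look-at pitch to BendAnimTarget.
; Otherwise, the Pivot sways on time-driven sine and cosine roll and pitch, and BendAnimTarget resets to zero.
; RotatePivotSlowly smooths both modes with RInterpTo on world rotation.
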(event EventTick
  (params (DeltaSeconds :type Float%20%28single-precision%29))
  (bind _returnvalue (Game|Player|GetPlayerPawn 0))
  (bind _returnvalue_2 (Transformation|GetActorLocation))
  (bind _returnvalue_3 (Actor|GetGameTimeSinceCreation))
  (bind _returnvalue_4 (Transformation|GetActorLocation _returnvalue))
  (bind _returnvalue_5 (Math|Rotator|FindLookatRotation _returnvalue_2 _returnvalue_4))
  (bind _output_get (Variables|Default|Setfollowing%20player (and (Variables|/Game/FrauHolle_Main/Blueprints/TriggerBP.TriggerBP_C|Gettriggered (Variables|Default|GetTrigger)) (Variables|/Game/FrauHolle_Main/Blueprints/Axt.Axt_C|GetLebendig (Variables|Default|GetAxt)))))
  (if _output_get
    (CallFunction|RotatePivotSlowly (Math|Rotator|MakeRotator 0.0 0.0 (.yaw _returnvalue_5)) 1.0)
    (Variables|Default|Setbend%20anim%20target (Math|Float|MapRangeClamped (.pitch _returnvalue_5) -6e+01 0.0 0.0 1.0))
    (else
      (CallFunction|RotatePivotSlowly (Math|Rotator|MakeRotator (* (Variables|Default|GetX%20swing%20amplitude) (Math|Trig|Sin(Radians) (* (Variables|Default|GetX%20swing%20speed) _returnvalue_3))) (* (Math|Trig|Cos(Radians) (* _returnvalue_3 (Variables|Default|GetY%20swing%20speed))) (Variables|Default|GetY%20swing%20amplitude)) 0.0) 1.0)
      (Variables|Default|Setbend%20anim%20target 0.0))))

(fn ConstructionScript)

(fn RotatePivotSlowly
  (params (TargetRot :type Rotator) (InterpSpeed :type Float%20%28single-precision%29))
  (bind _pivot (Variables|Default|GetPivot))
  (Transformation|SetWorldRotation _pivot (Math|Interpolation|RInterpTo (Transformation|GetWorldRotation _pivot) TargetRot (Utilities|Time|GetWorldDeltaSeconds) InterpSpeed) false false)
  (return))