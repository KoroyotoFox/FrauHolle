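; Exit trigger actor for the witch (Ausgang_Hexe) in the Frau Holle VR game that rewards the player with Karma.
; When the player pawn first overlaps it, it increments Karma on VRGameMode by one.
; The Abgeschlossen (completed) flag is then set, so the reward is granted only once.
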(event Collision|EventActorBeginOverlap
  (params (OtherActor :type Actor%20Object%20Reference))
  (if (and (== (Game|Player|GetPlayerPawn 0) OtherActor) (not (Variables|Default|GetAbgeschlossen)))
    (bind _asvrgame_mode (Utilities|Casting|CastToVRGameMode (Game|GetGameMode)))
    (Variables|/Game/FrauHolle_Main/Blueprints/VRGameMode.VRGameMode_C|SetKarma _asvrgame_mode (+ (Variables|/Game/FrauHolle_Main/Blueprints/VRGameMode.VRGameMode_C|GetKarma _asvrgame_mode) 1))
    (Variables|Default|SetAbgeschlossen true)))

(fn ConstructionScript)