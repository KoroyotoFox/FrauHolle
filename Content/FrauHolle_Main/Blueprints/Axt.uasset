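; Grabbable VR axe that lets the player strike the tree heart (Baumherz), at a cost in karma.
; Its GrabComponent events track whether it is held, and its mesh's rigid body starts asleep.
; A hit on Baumherz while held, with Lebendig set and AusgangBaum not yet completed, clears Lebendig, lowers the VRGameMode's Karma and marks AusgangBaum as Abgeschlossen (completed).
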(event OnGrabbed(GrabComponent)
  (Variables|Default|SetGegriffen true))

(event OnDropped(GrabComponent)
  (Variables|Default|SetGegriffen false))

(event EventBeginPlay
  (Class|PrimitiveComponent|PutRigidBodytoSleep (Variables|Default|GetStaticMesh) "None"))

(event Collision|EventHit
  (params (MyComp :type Primitive%20Component%20Object%20Reference) (Other :type Actor%20Object%20Reference) (OtherComp :type Primitive%20Component%20Object%20Reference) (bSelfMoved :type Boolean) (HitLocation :type Vector :default "0, 0, 0") (HitNormal :type Vector :default "0, 0, 0") (NormalImpulse :type Vector :default "0, 0, 0") (Hit :type Hit%20Result%20Structure%20%28by%20ref%29))
  (if (and (and (== Other "/Game/FrauHolle_Main/Blueprints/Baumherz.Baumherz") (Variables|Default|GetGegriffen)) (and (Variables|Default|GetLebendig) (not (Variables|/Game/FrauHolle_Main/Blueprints/Ausgang_Baum.Ausgang_Baum_C|GetAbgeschlossen (Variables|Default|GetAusgang%20Baum)))))
    (Variables|Default|SetLebendig false)
    (bind _asvrgame_mode (Utilities|Casting|CastToVRGameMode (Game|GetGameMode)))
    (Variables|/Game/FrauHolle_Main/Blueprints/VRGameMode.VRGameMode_C|SetKarma _asvrgame_mode (- (Variables|/Game/FrauHolle_Main/Blueprints/VRGameMode.VRGameMode_C|GetKarma _asvrgame_mode) 1))
    (Variables|/Game/FrauHolle_Main/Blueprints/Ausgang_Baum.Ausgang_Baum_C|SetAbgeschlossen (Variables|Default|GetAusgang%20Baum) true)))

(fn ConstructionScript
  (|CallParentFunction))